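; AI tank enemy that chases the player and dies when a Shell hits it.
; Tick drives movement input toward the player, switching back toward the spawn point recorded at BeginPlay while closer than a fixed distance.
; A Shell overlap on the capsule hides the mesh, plays explosion effects, grants the player health and destroys the tank, the last only if the MyCharacter cast succeeds.
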(event `self.CapsuleComponent.OnComponentBeginOverlap`
  (params (OtherActor :type "Actor Object Reference") (OtherComp :type "PrimitiveComponent Object Reference") (OtherBodyIndex :type Integer) (bFromSweep :type Boolean) (SweepResult :type "EngineTypes.HitResult Structure (by ref)"))
  (bind _returnvalue (`self.K2_GetActorLocation`))
  (cast `/Game/Blueprints/Shell` OtherActor)
  (`SceneComponent.SetHiddenInGame` (`self.Mesh`) true false)
  (`GameplayStatics.SpawnEmitterAtLocation` "/Game/StarterContent/Particles/P_Explosion.P_Explosion" _returnvalue)
  (`GameplayStatics.PlaySoundAtLocation` "/Game/Blueprints/kaboom.kaboom" _returnvalue 0.5)
  (bind _asmy_character (cast `/Game/Blueprints/MyCharacter` (`GameplayStatics.GetPlayerPawn` 0)))
  (`/Game/Blueprints/MyCharacter.Add Health` _asmy_character 10.0)
  (`self.K2_DestroyActor`))

(event `self.ReceiveTick`
  (params (DeltaSeconds :type "Float (single-precision)"))
  (if (`self.Too Close`)
    (`self.AddMovementInput` (`KismetMathLibrary.Normal` (- (`self.SpawnLocation`) (`self.K2_GetActorLocation`))))
    (else
      (`self.AddMovementInput` (`KismetMathLibrary.Normal` (- (`self.K2_GetActorLocation` (`GameplayStatics.GetPlayerPawn` 0)) (`self.K2_GetActorLocation`))))))
  (`/Engine/EditorBlueprintResources/StandardMacros.CompareFloat` (`KismetMathLibrary.VSize` (- (`self.K2_GetActorLocation` (`GameplayStatics.GetPlayerPawn` 0)) (`self.K2_GetActorLocation`))) 300.0
    (:`>`
      (set `self.Too Close` false))
    (:`<`
      (set `self.Too Close` true))))

(event `self.ReceiveBeginPlay`
  (set `self.SpawnLocation` (`self.K2_GetActorLocation`)))

(fn `UserConstructionScript`)